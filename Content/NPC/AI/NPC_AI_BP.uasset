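; NPC AI controller that starts patrol behavior and flags NPCs as aggroed when their perception updates.
; On begin play it loads the PatrolData blackboard and runs the Patrol behavior tree.
; Any target perception update prints a debug message, then writes the actor to AgroActor and sets IsAgro true.
; The handler does not filter by sense or sensing success, and never clears the aggro keys.
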(event OnTargetPerceptionUpdated(AIPerception)
  (params (Actor :type Actor%20Object%20Reference) (Stimulus :type AI%20Stimulus%20Structure))
  (bind _returnvalue (Class|AIPerceptionSystem|GetSenseClassforStimulus Stimulus))
  (Development|PrintString (Utilities|String|Append (Utilities|GetDisplayName (Pawn|GetControlledPawn)) "  " (Utilities|GetClassDisplayName _returnvalue) "  " (Utilities|GetDisplayName Actor)) true true "(R=0.000000,G=0.660000,B=1.000000,A=1.000000)" 5.0)
  ;[1 1 1] Trigger Agro flag and set the noticed actor to be the target
  (AI|Components|Blackboard|SetValueasObject (Variables|Default|GetBlackboard) (Utilities|Name|MakeLiteralName "AgroActor") Actor)
  (AI|Components|Blackboard|SetValueasBool (Variables|Default|GetBlackboard) (Utilities|Name|MakeLiteralName "IsAgro") true))

(event EventBeginPlay
  (Class|AIController|UseBlackboard "/Game/NPC/AI/PatrolData.PatrolData")
  (AI|RunBehaviorTree "/Game/NPC/AI/Patrol.Patrol"))

(fn ConstructionScript)